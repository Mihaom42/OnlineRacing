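; Spline actor in the environment that appears intended as a track path for race progress, though all its logic is currently disconnected.
; BeginPlay and the construction script do nothing.
; Unwired construction nodes would rebuild NewSplineComponent by resampling SplineComponent at fixed distance intervals in world space.
; Unwired event nodes would pass that spline and the player's BP_Vehicle to a WBP_RaceProgress widget on screen.
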(event `self.ReceiveBeginPlay`)

(fn `UserConstructionScript`)